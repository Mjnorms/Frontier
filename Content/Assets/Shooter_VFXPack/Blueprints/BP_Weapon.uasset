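; BP_Weapon is a VFX pack weapon that fires automatically in a timed loop after an initial delay, with no input handling.
; An optional Niagara indicator traces the aim line before each shot.
; Each shot spawns a classic or instant-hit projectile configured with trail, hit effect and decal color, plays the arm fire montage, and optionally triggers a muzzle flash.
; The construction script snaps the gun to the arms' GripPoint socket.
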(event Custom|Again
  (bind _arrow (Variables|Default|GetArrow))
  (bind _arrow_2 (Variables|Default|GetArrow))
  (bind _returnvalue (Math|Vector|GetForwardVector _arrow_2))
  (bind _returnvalue_2 (Transformation|GetWorldTransform _arrow))
  (bind _returnvalue_3 (* _returnvalue 3e+03))
  (bind _returnvalue_4 (+ (.location _returnvalue_2) _returnvalue_3))
  (Utilities|FlowControl|Delay (Variables|Default|GetDelay))
  (Class|NiagaraComponent|SetAsset (Variables|Default|GetMuzzleFlash) (Variables|Effect|GetMuzzleFlash_Effect) true)
  (if (Variables|Default|GetbIndicator)
    (bind _returnvalue_5 (Niagara|SpawnSystematLocation "/Game/Assets/Shooter_VFXPack/Particles/Projectiles/P_Trails_PARTS_Attraction_IH.P_Trails_PARTS_Attraction_IH" (.location _returnvalue_2) (.rotation _returnvalue_2)))
    (bind (_outhit _returnvalue_6) (Collision|LineTraceByChannel (.location _returnvalue_2) _returnvalue_4 "TraceTypeQuery1" false 0 "None" true "(R=1.000000,G=0.000000,B=0.000000,A=1.000000)" "(R=0.000000,G=1.000000,B=0.000000,A=1.000000)" 0.1))
    (if _returnvalue_6
      (Effects|Components|ParticleSystem|SetVectorParameter _returnvalue_5 "User.Hit" (.ImpactPoint (Collision|BreakHitResult _outhit)))
      (else
        (Effects|Components|ParticleSystem|SetVectorParameter _returnvalue_5 "User.Hit" _returnvalue_4)))
    (Utilities|FlowControl|Delay 0.6))
  (if (not (Variables|Default|GetbInstantHit))
    (Game|SpawnActorfromClass "/Game/Assets/Shooter_VFXPack/Blueprints/BP_Projectile_Classic.BP_Projectile_Classic_C" (Transformation|GetWorldTransform (Variables|Default|GetArrow)) "Undefined" "OverrideRootScale" 0 (Variables|Default|GetInitial%20Speed) (Variables|Default|GetbGravity%20Enabled) (Variables|Effect|GetNiagara_Trail) (Variables|Effect|GetNiagara_Hit) (Variables|Effect|GetbMuzzleFlashAndHit) (Variables|Effect|GetbImpact%20Normal) (Variables|Default|GetDecalEmissive%20Color) 0)
    (else
      (Game|SpawnActorfromClass "/Game/Assets/Shooter_VFXPack/Blueprints/BP_Projectile_InstantHit.BP_Projectile_InstantHit_C" (Transformation|GetWorldTransform (Variables|Default|GetArrow)) "Undefined" "OverrideRootScale" 0 2e+03 true (Variables|Effect|GetbMuzzleFlashAndHit) (Variables|Effect|GetNiagara_Trail) (Variables|Effect|GetNiagara_Hit) (Variables|Effect|GetbImpact%20Normal) (Variables|Default|GetDecalEmissive%20Color) 0)))
  (Animation|Montage|MontagePlay (Components|SkeletalMesh|GetAnimInstance (Variables|Default|GetSkeletalMesh)) "/Game/Assets/Shooter_VFXPack/DEMO/Character_02/Animations/FirstPersonFire_Montage.FirstPersonFire_Montage" 1.0 "MontageLength" 0.0 true) ; Play animation on arm mesh
  (CallFunction|Again)
  (if (Variables|Effect|GetbMuzzleFlashAndHit)
    (Components|Activation|Activate (Variables|Default|GetMuzzleFlash) true)))

(event EventBeginPlay
  (bind _arrow (Variables|Default|GetArrow))
  (bind _arrow_2 (Variables|Default|GetArrow))
  (bind _returnvalue (Math|Vector|GetForwardVector _arrow_2))
  (bind _returnvalue_2 (Transformation|GetWorldTransform _arrow))
  (bind _returnvalue_3 (* _returnvalue 3e+03))
  (bind _returnvalue_4 (+ (.location _returnvalue_2) _returnvalue_3))
  (Utilities|FlowControl|Delay (Variables|Default|GetInitialDelay))
  (Class|NiagaraComponent|SetAsset (Variables|Default|GetMuzzleFlash) (Variables|Effect|GetMuzzleFlash_Effect) true)
  (if (Variables|Default|GetbIndicator)
    (bind _returnvalue_5 (Niagara|SpawnSystematLocation "/Game/Assets/Shooter_VFXPack/Particles/Projectiles/P_Trails_PARTS_Attraction_IH.P_Trails_PARTS_Attraction_IH" (.location _returnvalue_2) (.rotation _returnvalue_2)))
    (bind (_outhit _returnvalue_6) (Collision|LineTraceByChannel (.location _returnvalue_2) _returnvalue_4 "TraceTypeQuery1" false 0 "None" true "(R=1.000000,G=0.000000,B=0.000000,A=1.000000)" "(R=0.000000,G=1.000000,B=0.000000,A=1.000000)" 0.1))
    (if _returnvalue_6
      (Effects|Components|ParticleSystem|SetVectorParameter _returnvalue_5 "User.Hit" (.ImpactPoint (Collision|BreakHitResult _outhit)))
      (else
        (Effects|Components|ParticleSystem|SetVectorParameter _returnvalue_5 "User.Hit" _returnvalue_4)))
    (Utilities|FlowControl|Delay 0.6))
  (if (not (Variables|Default|GetbInstantHit))
    (Game|SpawnActorfromClass "/Game/Assets/Shooter_VFXPack/Blueprints/BP_Projectile_Classic.BP_Projectile_Classic_C" (Transformation|GetWorldTransform (Variables|Default|GetArrow)) "Undefined" "OverrideRootScale" 0 (Variables|Default|GetInitial%20Speed) (Variables|Default|GetbGravity%20Enabled) (Variables|Effect|GetNiagara_Trail) (Variables|Effect|GetNiagara_Hit) (Variables|Effect|GetbMuzzleFlashAndHit) (Variables|Effect|GetbImpact%20Normal) (Variables|Default|GetDecalEmissive%20Color) 0)
    (else
      (Game|SpawnActorfromClass "/Game/Assets/Shooter_VFXPack/Blueprints/BP_Projectile_InstantHit.BP_Projectile_InstantHit_C" (Transformation|GetWorldTransform (Variables|Default|GetArrow)) "Undefined" "OverrideRootScale" 0 2e+03 true (Variables|Effect|GetbMuzzleFlashAndHit) (Variables|Effect|GetNiagara_Trail) (Variables|Effect|GetNiagara_Hit) (Variables|Effect|GetbImpact%20Normal) (Variables|Default|GetDecalEmissive%20Color) 0)))
  (Animation|Montage|MontagePlay (Components|SkeletalMesh|GetAnimInstance (Variables|Default|GetSkeletalMesh)) "/Game/Assets/Shooter_VFXPack/DEMO/Character_02/Animations/FirstPersonFire_Montage.FirstPersonFire_Montage" 1.0 "MontageLength" 0.0 true) ; Play animation on arm mesh
  (CallFunction|Again)
  (if (Variables|Effect|GetbMuzzleFlashAndHit)
    (Components|Activation|Activate (Variables|Default|GetMuzzleFlash) true)))

(fn ConstructionScript
  (Transformation|AttachComponentToComponent (Variables|Default|GetFP_Gun) (Variables|Default|GetSkeletalMesh) "GripPoint" "SnapToTarget" "SnapToTarget" "SnapToTarget" true))