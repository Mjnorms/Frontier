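; Instant-hit (hitscan) projectile actor that resolves its impact on BeginPlay with a forward Visibility line trace instead of moving.
; A Niagara trail receives the impact point, or the max-range point on a miss, through its User.Hit parameter.
; If enabled, a hit effect spawns facing either the surface normal, with a randomly scaled emissive decal, or back toward the trace start.
; The actor destroys itself after a short delay.
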(event EventBeginPlay
  (bind _returnvalue (Transformation|GetActorLocation))
  (bind _returnvalue_2 (Transformation|GetActorForwardVector))
  (bind _trail (Variables|Default|GetTrail))
  (bind _distancemax (Variables|Default|GetDistanceMax))
  (bind _returnvalue_3 (* _returnvalue_2 _distancemax))
  (bind _returnvalue_4 (+ _returnvalue _returnvalue_3))
  (Class|NiagaraComponent|SetAsset (Variables|Default|GetTrail) (Variables|Default|GetNiagara_Trail) true)
  (bind (_outhit _returnvalue_5) (Collision|LineTraceByChannel _returnvalue _returnvalue_4 "TraceTypeQuery1" false 0 "None" true "(R=1.000000,G=0.000000,B=0.000000,A=1.000000)" "(R=0.000000,G=1.000000,B=0.000000,A=1.000000)" 0.1))
  (if _returnvalue_5
    (Effects|Components|ParticleSystem|SetVectorParameter _trail "User.Hit" (.ImpactPoint (Collision|BreakHitResult _outhit)))
    (Utilities|FlowControl|Sequence
      (:then_0
        (if (Variables|Default|GetbHit)
          (if (Variables|Default|GetbImpactNormal)
            (Niagara|SpawnSystematLocation (Variables|Default|GetHitEffect) (.ImpactPoint (Collision|BreakHitResult _outhit)) (Math|Rotator|MakeRotfromX (.ImpactNormal (Collision|BreakHitResult _outhit))))
            (Game|SpawnActorfromClass "/Game/Assets/Shooter_VFXPack/Blueprints/BP_DecalHit.BP_DecalHit_C" (Math|Transform|MakeTransform (.ImpactPoint (Collision|BreakHitResult _outhit)) (Math|Rotator|MakeRotfromZ (.ImpactNormal (Collision|BreakHitResult _outhit))) (Math|Conversions|ToVector(Float) (Math|Random|RandomFloatinRange 0.6 0.95))) "Undefined" "OverrideRootScale" 0 1.5 1.0 false 0.0 (Variables|Default|GetEmissive%20Color) 0)
            (else
              (Niagara|SpawnSystematLocation (Variables|Default|GetHitEffect) (.ImpactPoint (Collision|BreakHitResult _outhit)) (Math|Rotator|MakeRotfromX (- (.TraceStart (Collision|BreakHitResult _outhit)) (.ImpactPoint (Collision|BreakHitResult _outhit)))))))))
      (:then_1
        (Utilities|FlowControl|Delay 5.0 :!label _label)
        (Actor|DestroyActor)))
    (else
      (Effects|Components|ParticleSystem|SetVectorParameter _trail "User.Hit" _returnvalue_4)
      (goto _label))))

(fn ConstructionScript)